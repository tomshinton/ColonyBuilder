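; BP_TestWall is a prototype building wall that rises from the ground up when it spawns.
; BeginPlay flattens MeshComponent to zero Z scale and picks a random GrowthRate, so each instance grows at its own speed.
; Tick eases the mesh toward full scale with VInterpTo, using GrowthRate as the interp speed, and keeps running with no completion check.
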(event `self.ReceiveBeginPlay`
  (`SceneComponent.SetWorldScale3D` (`self.MeshComponent`) (1.0 1.0 0.0))
  (set `self.GrowthRate` (`KismetMathLibrary.RandomFloatInRange` 0.5 1.0)))

(event `self.ReceiveTick`
  (params (DeltaSeconds :type "Float (single-precision)"))
  (`SceneComponent.SetWorldScale3D` (`self.MeshComponent`) (`KismetMathLibrary.VInterpTo` (`SceneComponent.RelativeScale3D` (`self.MeshComponent`)) (1.0 1.0 1.0) DeltaSeconds (`self.GrowthRate`))))

(fn `UserConstructionScript`
  (`parent.UserConstructionScript`))
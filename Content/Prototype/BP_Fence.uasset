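; Prototype fence actor that builds a fence along a spline in the construction script.
; Spline mesh segments of the fence mesh bend along the curve, each spanning the mesh's X bounds extent.
; At every second segment step, a downward trace places a post slightly below the hit point, rotated to the spline's yaw only.
; Each post gets its own hierarchical instanced static mesh component.
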(fn `UserConstructionScript`
  (bind _spline (`self.Spline`))
  (bind _spline_2 (`self.Spline`))
  (bind (_returnvalue_origin _returnvalue_boxextent) (`KismetMathLibrary.BreakBoxSphereBounds` (`StaticMesh.GetBounds` (`self.FenceMesh`))))
  (bind (_returnvalue_origin_2 _returnvalue_boxextent_2) (`KismetMathLibrary.BreakBoxSphereBounds` (`StaticMesh.GetBounds` (`self.FenceMesh`))))
  (bind _x (.x _returnvalue_boxextent))
  (bind _x_2 (.x _returnvalue_boxextent_2))
  (for _index (range (+ (`KismetMathLibrary.FTrunc` (/ (`SplineComponent.GetSplineLength` (`self.Spline`)) _x_2)) 1))
    (bind _returnvalue (`AddComponent|NODE_AddSplineMeshComponent-0`))
    (`StaticMeshComponent.SetStaticMesh` _returnvalue (`self.FenceMesh`))
    (`SceneComponent.K2_AttachToComponent` _returnvalue (`self.DefaultSceneRoot`) "None" "KeepRelative" "KeepRelative" "KeepRelative" true)
    (bind _returnvalue_2 (* _index _x_2))
    (bind _returnvalue_3 (+ _returnvalue_2 _x_2))
    (`SplineMeshComponent.SetStartAndEnd` _returnvalue (`SplineComponent.GetLocationAtDistanceAlongSpline` _spline _returnvalue_2 "Local") (`SplineComponent.GetTangentAtDistanceAlongSpline` (`self.Spline`) _returnvalue_2 "Local") (`SplineComponent.GetLocationAtDistanceAlongSpline` _spline _returnvalue_3 "Local") (`SplineComponent.GetTangentAtDistanceAlongSpline` (`self.Spline`) _returnvalue_3 "Local") true))
  (for _index_2 (range (+ (`KismetMathLibrary.FTrunc` (/ (/ (`SplineComponent.GetSplineLength` (`self.Spline`)) _x) 2.0)) 1))
    (bind _returnvalue_4 (`AddComponent|NODE_AddHierarchicalInstancedStaticMeshComponent-0`))
    (bind _returnvalue_5 (* (* _index_2 2.0) _x))
    (bind _returnvalue_6 (`SplineComponent.GetLocationAtDistanceAlongSpline` _spline_2 _returnvalue_5 "World"))
    (bind _outhit (`KismetSystemLibrary.LineTraceSingle` (+ _returnvalue_6 (0.0 0.0 100.0)) (- _returnvalue_6 (0.0 0.0 1000.0)) "TraceTypeQuery1"))
    (`SceneComponent.K2_AttachToComponent` _returnvalue_4 (`self.DefaultSceneRoot`) "None" "KeepRelative" "KeepRelative" "KeepRelative" true)
    (`StaticMeshComponent.SetStaticMesh` _returnvalue_4 (`self.PostMesh`))
    (bind (_returnvalue_roll _returnvalue_pitch _returnvalue_yaw) (`KismetMathLibrary.BreakRotator` (`SplineComponent.GetRotationAtDistanceAlongSpline` _spline_2 _returnvalue_5 "World")))
    (`InstancedStaticMeshComponent.AddInstanceWorldSpace` _returnvalue_4 (`KismetMathLibrary.MakeTransform` (- (`.Location` (`GameplayStatics.BreakHitResult` _outhit)) (0.0 0.0 10.0)) (`KismetMathLibrary.MakeRotator` 0.0 0.0 _returnvalue_yaw)))))